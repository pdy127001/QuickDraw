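; BP_Samurai is a 2D sprite duelist that slides in on BeginPlay and plays a lunge attack when PlayAttackAnim is called.
; Timelines lerp the sprite from a start offset to its cached position, and from local origin to AttackPos for attacks.
; A mid-attack timeline event swaps to the tanuki attack sprite and notifies BP_QD_GameModeBase, passing whether the pawn is player-controlled.
; The Defeated event is an empty stub.
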(event Custom|SlideIn
  (Components|Timeline|SetPlayRate (Variables|Default|GetSlideInAnim) 2.0)
  (bind _alpha (Timeline|SlideInAnim PlayFromStart)
    (:Update
      (Transformation|SetRelativeLocation (Variables|Default|GetPaperSprite) (Math|Vector|Lerp(Vector) (Variables|Default|GetSlide%20Start%20Pos) (Variables|Default|GetSpriteDefaultPos) _alpha) false false))))

(event EventBeginPlay
  (Variables|Default|SetSpriteDefaultPos (Variables|/Script/Engine.SceneComponent|GetRelativeLocation (Variables|Default|GetPaperSprite)))
  (CallFunction|Slidein))

(event Collision|EventActorBeginOverlap
  (params (OtherActor :type Actor%20Object%20Reference)))

(event EventTick
  (params (DeltaSeconds :type Float%20%28single-precision%29)))

(event EventPlayAttackAnim
  (Components|Timeline|SetPlayRate (Variables|Default|GetAttackAnim) 8.0)
  (bind _alpha (Timeline|AttackAnim PlayFromStart)
    (:Update
      (Transformation|SetRelativeLocation (Variables|Default|GetPaperSprite) (Math|Vector|Lerp(Vector) "0, 0, 0" (Variables|/Script/Engine.SceneComponent|GetRelativeLocation (Variables|Default|GetAttackPos)) _alpha) false false))
    (:ChangeSprite
      (CallFunction|AttackMotion)
      (bind _asbp_qd_game_mode_base (Utilities|Casting|CastToBP_QD_GameModeBase (Game|GetGameMode)))
      (Default|AttackedSuccesfully _asbp_qd_game_mode_base (Pawn|IsPlayerControlled)))))

(event EventDefeated)

(fn ConstructionScript)

(fn AttackMotion
  (Rendering|Components|Sprite|SetSprite (Variables|Default|GetPaperSprite) "/Game/Quick_Draw_Assets/Tanuki/T_Tanuki_Attack_Sprite.T_Tanuki_Attack_Sprite"))